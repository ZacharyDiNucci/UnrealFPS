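; BP_TPWeapon is the third-person weapon actor, handling pickup, hitscan firing and effects for other players.
; On authority, capsule overlap hands rifles to players lacking one and disables physics and collision; the pistol branch is unfinished.
; Server_FireWeapon traces from the supplied camera view and applies point damage scaled by the hit body part's physical surface.
; Multi_Effects plays muzzle flash and sound, skipping the owner's own view via a player-pawn check.
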(event OnComponentBeginOverlap(Capsule)
  (params (OverlappedComponent :type Primitive%20Component%20Object%20Reference) (OtherActor :type Actor%20Object%20Reference) (OtherComp :type Primitive%20Component%20Object%20Reference) (OtherBodyIndex :type Integer) (bFromSweep :type Boolean) (SweepResult :type Hit%20Result%20Structure%20%28by%20ref%29))
  (Networking|SwitchHasAuthority
    (:Authority
      (if (Actor|ActorHasTag OtherActor "Player")
        (if (Variables|Default|GetIsRifle)
          (bind _hasrifle (Class|INTBaseCharacter|CheckforRifle(Message) OtherActor))
          (if (not _hasrifle)
            (CallFunction|EquipRifle)
            (Class|INTBaseCharacter|EquipRifle(Message) OtherActor (Variables|Default|GetWeaponInfo) self))
          (else
            (bind _haspistol (Class|INTBaseCharacter|CheckforPistol(Message) OtherActor))
            (if _haspistol
              _)))))))

(event Custom|EquipRifle
  (bind _weapon (Variables|Default|GetWeapon))
  (Physics|SetEnableGravity _weapon false)
  (Physics|SetSimulatePhysics _weapon false)
  (Collision|SetCollisionEnabled _weapon "NoCollision")
  (Collision|SetCollisionEnabled (Variables|Default|GetCapsule) "NoCollision"))

(event Custom|Server_FireWeapon
  (params (CameraLocation :type Vector) (CameraRotation :type Rotator))
  (Variables|Default|SetShooting%20Location CameraLocation)
  (Variables|Default|SetShooting%20Rotation CameraRotation)
  (bind (_outhit _returnvalue) (Collision|LineTraceByChannel (Variables|Default|GetShooting%20Location) (+ (Variables|Default|GetShooting%20Location) (* (Math|Vector|GetForwardVector (Variables|Default|GetShooting%20Rotation)) (Variables|Default|Getrange))) "TraceTypeQuery1" false (Utilities|Array|MakeArray (Components|GetOwner) self) "ForDuration"))
  (if _returnvalue
    (switch Utilities|FlowControl|Switch|SwitchonEPhysicalSurface (Variables|/Script/PhysicsCore.PhysicalMaterial|GetSurfaceType (.PhysMat (Collision|BreakHitResult _outhit)))
      (:SurfaceType1
        (Utilities|DamagePlayer (.HitActor (Collision|BreakHitResult _outhit)) _outhit (* (Variables|Default|GetDamage) 2.5)))
      (:SurfaceType2
        (Utilities|DamagePlayer (.HitActor (Collision|BreakHitResult _outhit)) _outhit (Variables|Default|GetDamage)))
      (:SurfaceType3
        (Utilities|DamagePlayer (.HitActor (Collision|BreakHitResult _outhit)) _outhit (* (Variables|Default|GetDamage) 0.9)))
      (:SurfaceType4
        (Utilities|DamagePlayer (.HitActor (Collision|BreakHitResult _outhit)) _outhit (* (Variables|Default|GetDamage) 0.7))))))

(event Custom|Multi_Effects
  (if (not (== (Components|GetOwner) (Game|Player|GetPlayerPawn 0)))
    (Effects|SpawnEmitterAttached (Variables|Default|GetMuzzleflash) (Variables|Default|GetWeapon) "MuzzleFlash")
    (Audio|PlaySoundatLocation (Variables|Default|GetFireSound) (Transformation|GetActorLocation) "0, 0, 0" 1.0 1.0 0.0 0 0 0)))

(fn ConstructionScript)